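; BEnemy is an enemy Blueprint that can take damage and be destroyed.
; Any damage is passed to its Health component, and the actor destroys itself once current health reaches zero or below.
; Surviving hits print the remaining health and the damage amount to the screen.
; On BeginPlay it stores the first player pawn as Target, which this Blueprint's graphs do not use further.
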(event `self.ReceiveAnyDamage`
  (params (Damage :type "Float (single-precision)") (DamageType :type "DamageType Object Reference") (InstigatedBy :type "Controller Object Reference") (DamageCauser :type "Actor Object Reference"))
  (bind _health (`self.Health`))
  (bind _currenthealth (`HealthComponent.currentHealth` _health))
  (`HealthComponent.ModifyHealth` _health Damage false)
  (if (<= _currenthealth 0.0)
    (`self.K2_DestroyActor`)
    (else
      (`KismetSystemLibrary.PrintString` (`KismetStringLibrary.Conv_DoubleToString` _currenthealth) true true (struct :`G` 0.66 :`B` 1.0 :`A` 1.0) 0.5)
      (`KismetSystemLibrary.PrintString` (`KismetStringLibrary.Concat_StrStr` "Damage: " (`KismetStringLibrary.Conv_DoubleToString` Damage))))))

(event `self.ReceiveBeginPlay`
  ;[1 1 1] Initialize Tracking
  (set `self.target` (`GameplayStatics.GetPlayerPawn` 0)))

(fn `UserConstructionScript`)