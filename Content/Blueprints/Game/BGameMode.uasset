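; Game mode that handles initial spawning and timed respawning of enemies.
; On game start it spreads the configured enemy classes round-robin across the enemy spawners.
; Killed enemies join a respawn list and start their own timer, which Tick polls through CanRespawn.
; A ready enemy leaves the list, a fresh instance of its class spawns at a random spawner, and the old actor is destroyed.
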(event `self.ReceiveTick`
  (params (DeltaSeconds :type "Float (single-precision)"))
  (`self.Process Enemy Respawns`))

(event `Process Enemy Respawns`
  (for _array_element (`self.Respawning Enemies`)
    (if (`EnemyPawn.CanRespawn` _array_element)
      (`self.Respawn Enemies` _array_element))))

(event `self.OnGameStart`
  (`|ExecutionSequence`
    (:`then_0`
      ;[1 1 1] Checks if Enemy Spawners are present in the level
      (if (not (>= (`KismetArrayLibrary.Array_Length` (`self.Enemy Spawners`)) 0))
        (`KismetSystemLibrary.PrintString` "There are no Enemy Spawners in the current level")))
    (:`then_1`
      (`self.Spawn Enemies` (`self.Enemy Spawners`) (`self.Enemies Characters`)))))

(event `self.OnCharacterKilled`
  (params (KilledEnemy :type "EnemyPawn Object Reference"))
  (`KismetArrayLibrary.Array_Add` (`self.Respawning Enemies`) KilledEnemy)
  (`EnemyPawn.StartRespawnTimer` KilledEnemy (`self.Respawn Timer`)))

(fn `Respawn Enemies`
  (params (`Enemy To Respawn` :type "EnemyPawn Object Reference"))
  (set `self.Enemy To Respawn` `Enemy To Respawn`)
  (`|ExecutionSequence`
    (:`then_0`
      (`KismetArrayLibrary.Array_RemoveItem` (`self.Respawning Enemies`) (`self.Enemy To Respawn`)))
    (:`then_1`
      (`self.Spawn Enemy` (`self.Enemy To Respawn`) (`self.Enemy Spawners`)))
    (:`then_2`
      (`self.K2_DestroyActor` (`self.Enemy To Respawn`)))))

(fn `Spawn Enemies`
  (params (Spawners :type "Array of /Game/Blueprints/Enemy/BEnemy_Spawner Object Reference") (`Enemies To Spawn` :type "Array of /Game/Blueprints/Enemy/BEnemy Class Reference"))
  (for (_array_element _array_index) `Enemies To Spawn`
    (`EnemySpawner.SpawnEnemy` (`|GetArrayItem` Spawners (mod _array_index (`KismetArrayLibrary.Array_Length` Spawners))) _array_element))
  (return))

(fn `Spawn Enemy`
  (params (Enemy :type "EnemyPawn Object Reference") (Spawner :type "Array of /Game/Blueprints/Enemy/BEnemy_Spawner Object Reference"))
  (returns (`New Enemy` :type "EnemyPawn Object Reference"))
  (`EnemySpawner.SpawnEnemy` (`|GetArrayItem` Spawner (`KismetMathLibrary.RandomIntegerInRange` 0 (- (`KismetArrayLibrary.Array_Length` Spawner) 1))) (`GameplayStatics.GetObjectClass` Enemy))
  (return Enemy))

(fn `UserConstructionScript`)