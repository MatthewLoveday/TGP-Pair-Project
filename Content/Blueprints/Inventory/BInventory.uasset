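; Inventory Blueprint that holds an items array and drives its on-screen inventory UI, seeding the array with a constructed ammo item on BeginPlay.
; UpdateWidgetAppearance lazily fetches the widget from Ship_HUD, then shows or hides it along with the mouse cursor and mouse-over events.
; When shown, each item is assigned to the slot matching its array index and its image is refreshed.
; The pickup button handler only prints a message.
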(event `self.UpdateWidgetAppearance`
  (bind _returnvalue (`GameplayStatics.GetPlayerController` 0))
  (bind _uireference (`self.UIReference`))
  ;[1 1 1] Determine if ui reference is valid
  (if (not (`KismetSystemLibrary.IsValid` (`self.UIReference`)))
    (`self.GetUIReference`))
  ;[1 1 1] Set Blueprint Visbility
  (if (`self.UIVisible`)
    (`Widget.SetVisibility` _uireference "Visible")
    ;[1 1 1] Lock / Unlock mouse cursor
    (set `PlayerController.bShowMouseCursor` true _returnvalue)
    (set `PlayerController.bEnableMouseOverEvents` true _returnvalue)
    ;[1 1 1] Set Icons
    (for (_array_element _array_index) (`self.ItemsArray`)
      (bind _newparam (`/Game/Blueprints/UIs_HUDs/Inventory/InventoryBlueprint.GetInventoryItemFromArrayID` (`/Game/Blueprints/UIs_HUDs/Inventory/InventoryUI.InventoryBlueprint` (`self.UIReference`)) _array_index))
      (bind _asbitem_base (cast `/Game/Blueprints/Inventory/BItemBase` _array_element))
      (`/Game/Blueprints/UIs_HUDs/Inventory/InventoryItem.SetItem` _newparam _asbitem_base)
      (`/Game/Blueprints/UIs_HUDs/Inventory/InventoryItem.Update Item Image` _newparam))
    (else
      (`Widget.SetVisibility` _uireference "Hidden")
      (set `PlayerController.bShowMouseCursor` false _returnvalue)
      (set `PlayerController.bEnableMouseOverEvents` false _returnvalue))))

(event `UIButtonClick`
  (params (`Inventory Item` :type "/Game/Blueprints/UIs_HUDs/Inventory/InventoryItem Object Reference"))
  ;[1 1 1] Pickup UI Button
  (`KismetSystemLibrary.PrintString` "Pickup Item"))

(event `self.ReceiveBeginPlay`
  (bind _returnvalue (`|GenericCreateObject` "/Game/Blueprints/Inventory/BItemAmmo.BItemAmmo_C" self))
  (`KismetArrayLibrary.Array_Add` (`self.ItemsArray`) _returnvalue))

(fn `GetUIReference`
  (bind _asship_hud (cast `/Game/Blueprints/UIs_HUDs/Ship_HUD` (`PlayerController.GetHUD` (`GameplayStatics.GetPlayerController` 0))))
  (set `self.UIReference` (`/Game/Blueprints/UIs_HUDs/Ship_HUD.Inventory UI` _asship_hud)))