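; Rapid-fire pickup that temporarily removes the weapon cooldown of the player ship that collects it.
; On activation it caches the cooldown time from the ship's WeaponBase, sets it to zero and plays a reload sound.
; After an EffectTimer delay it restores the cached value.
; Tick spins the pickup around its yaw axis at a constant rate.
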(event `self.OnActivate`
  (params (pickedUpBy :type "Actor Object Reference"))
  (bind _asbplayer_ship (cast `/Game/Blueprints/Ship/BPlayerShip` pickedUpBy))
  (bind _weaponbase (`SpaceHarvestShooterPawn.weaponBase` _asbplayer_ship))
  (set `self.Temp CD Timer` (`WeaponBaseComponent.CoolDownTime` _weaponbase))
  (set `WeaponBaseComponent.CoolDownTime` 0.0 _weaponbase)
  (`GameplayStatics.PlaySound2D` "/Game/TwinStick/Audio/Reload.Reload" 1.0 1.0 0.0 null null)
  (`KismetSystemLibrary.Delay` (`self.Effect Timer`))
  (set `WeaponBaseComponent.CoolDownTime` (`self.Temp CD Timer`) _weaponbase))

(event `self.ReceiveTick`
  (params (DeltaSeconds :type "Float (single-precision)"))
  (`self.K2_SetActorRotation` (`KismetMathLibrary.MakeRotator` (.roll (`self.K2_GetActorRotation`)) (.pitch (`self.K2_GetActorRotation`)) (+ (.yaw (`self.K2_GetActorRotation`)) (* DeltaSeconds 80.0)))))

(fn `UserConstructionScript`)