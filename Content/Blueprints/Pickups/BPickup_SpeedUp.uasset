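; Speed boost pickup that temporarily multiplies the thrust of the ship controller belonging to whoever collects it.
; On activation it casts the instigator controller to BShipController, plays a 2D sound, multiplies Thrust by SpeedMultiplier, then divides it back after an EffectTimer delay.
; Debug strings print the boosted thrust and the end of the boost.
; Tick spins the pickup steadily around yaw.
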(event `self.OnActivate`
  (params (pickedUpBy :type "Actor Object Reference"))
  (bind _asbship_controller (cast `/Game/Blueprints/Ship/BShipController` (`self.GetInstigatorController` pickedUpBy)))
  (`GameplayStatics.PlaySound2D` "/Game/TwinStick/Audio/Speed.Speed" 1.0 1.0 0.0 null null)
  (bind _output_get (set `ShipController.Thrust` (* (`ShipController.Thrust` _asbship_controller) (`self.Speed Multiplier`)) _asbship_controller))
  (`KismetSystemLibrary.PrintString` (`KismetStringLibrary.Conv_DoubleToString` _output_get))
  (`KismetSystemLibrary.Delay` (`self.Effect Timer`))
  (set `ShipController.Thrust` (/ _output_get (`self.Speed Multiplier`)) _asbship_controller)
  (`KismetSystemLibrary.PrintString` "Boost Ended"))

(event `self.ReceiveTick`
  (params (DeltaSeconds :type "Float (single-precision)"))
  (`self.K2_SetActorRotation` (`KismetMathLibrary.MakeRotator` (.roll (`self.K2_GetActorRotation`)) (.pitch (`self.K2_GetActorRotation`)) (+ (.yaw (`self.K2_GetActorRotation`)) (* DeltaSeconds 80.0)))))

(fn `UserConstructionScript`)