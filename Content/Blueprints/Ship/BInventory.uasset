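; BInventory is a ship inventory Blueprint that links to the inventory UI on the player's HUD.
; On BeginPlay it casts player 0's HUD to Ship_HUD and caches its InventoryUI widget.
; Every Tick it branches on UIVisible, but both branches set the widget to Visible, so the flag has no effect and the UI is never hidden here.
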(event `self.ReceiveBeginPlay`
  (bind _asship_hud (cast `/Game/Blueprints/UIs_HUDs/Ship_HUD` (`PlayerController.GetHUD` (`GameplayStatics.GetPlayerController` 0))))
  (set `self.UIReference` (`/Game/Blueprints/UIs_HUDs/Ship_HUD.Inventory UI` _asship_hud)))

(event `self.ReceiveTick`
  (params (DeltaSeconds :type "Float (single-precision)"))
  (bind _uireference (`self.UIReference`))
  (if (`self.UIVisible`)
    (`Widget.SetVisibility` _uireference "Visible")
    (else
      (`Widget.SetVisibility` _uireference "Visible"))))